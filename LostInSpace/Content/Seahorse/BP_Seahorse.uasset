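; BP_Seahorse is a sprite-based seahorse that follows a target actor assigned through SetTarget.
; Each Tick, while the target is valid and at least StopFollowRange away, it sets CharacterMovement velocity straight toward it at max speed.
; During that movement it mirrors the sprite by flipping the sign of its world X scale according to the target's horizontal direction.
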(event EventBeginPlay)

(event Collision|EventActorBeginOverlap
  (params (OtherActor :type Actor%20Object%20Reference)))

(event EventTick
  (params (DeltaSeconds :type Float%20%28single-precision%29))
  (bind _returnvalue (Transformation|GetActorLocation))
  (bind _targettofollow (Variables|Default|GetTargetToFollow))
  (bind _sprite (Variables|Default|GetSprite))
  (bind _charactermovement (Variables|Character|GetCharacterMovement))
  (bind _returnvalue_2 (Transformation|GetActorLocation _targettofollow))
  (bind _returnvalue_3 (- _returnvalue_2 _returnvalue))
  (Utilities|IsValid _targettofollow
    (:Is%20Valid
      (if (<= (Variables|Default|GetStopFollowRange) (Math|Vector|VectorLength _returnvalue_3))
        (Variables|/Script/Engine.MovementComponent|SetVelocity _charactermovement (* (Math|Vector|Normalize _returnvalue_3) (Class|MovementComponent|GetMaxSpeed _charactermovement)))
        (if (< (.X (Math|Vector|BreakVector _returnvalue_3)) 0.0)
          (Transformation|SetWorldScale3D _sprite "2.000000,2.000000,2.000000")
          (else
            (Transformation|SetWorldScale3D _sprite "-2.000000,2.000000,2.000000")))))))

(fn ConstructionScript)

(fn SetTarget
  (params (ActorToFollow :type Actor%20Object%20Reference))
  (Variables|Default|SetTargetToFollow ActorToFollow))