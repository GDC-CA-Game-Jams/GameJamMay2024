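; BP_WordGameOnlyPawn is a player pawn that, on BeginPlay, starts background music, opens the main menu and enables mouse-driven UI input.
; The menu is pushed as a HUD onto the LISPlayerController's BaseUI.
; Two events crossfade word-game music in or out by stepping the BGM's "PuzzleGameFade" parameter, re-calling themselves after short delays until reaching the limit.
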(event Custom|FadeOutWordGameMusic
  (bind _output_get (Variables|Default|SetWordGameFadeValue (- (Variables|Default|GetWordGameFadeValue) 0.05)))
  (Audio|Parameter|SetFloatParameter (Variables|Default|GetBGM) "PuzzleGameFade" _output_get :!class /Script/AudioExtensions.AudioParameterControllerInterface)
  (if (<= _output_get 0.0)
    (Variables|Default|SetWordGameFadeValue 0.0)
    (else
      (Utilities|FlowControl|Delay 0.1)
      (CallFunction|FadeOutWordGameMusic))))

(event Custom|FadeInWordGameMusic
  (bind _output_get (Variables|Default|SetWordGameFadeValue (+ (Variables|Default|GetWordGameFadeValue) 0.05)))
  (Audio|Parameter|SetFloatParameter (Variables|Default|GetBGM) "PuzzleGameFade" _output_get :!class /Script/AudioExtensions.AudioParameterControllerInterface)
  (if (>= _output_get 1.0)
    (Variables|Default|SetWordGameFadeValue 1.0)
    (else
      (Utilities|FlowControl|Delay 0.1)
      (CallFunction|FadeinWordGameMusic))))

(event EventBeginPlay
  (bind _returnvalue (Game|GetPlayerController 0))
  (Audio|Components|Audio|Play (Variables|Default|GetBGM) 0.0)
  (Audio|Components|Audio|FadeIn (Variables|Default|GetBGM) 3.0 1.0 0.0 "Linear" :!class /Script/Engine.AudioComponent)
  (bind _aslisplayer_controller (Utilities|Casting|CastToLISPlayerController (Game|GetPlayerController 0)))
  (Class|BaseUI|PushHUD (Variables|/Script/LostInSpace.LISPlayerController|GetBaseUI _aslisplayer_controller) "/Game/UI/BP_MainMenu.BP_MainMenu_C")
  (Input|SetInputModeGameandUI _returnvalue 0 "DoNotLock" true false)
  (Variables|/Script/Engine.PlayerController|SetbShowMouseCursor _returnvalue true))

(event Collision|EventActorBeginOverlap
  (params (OtherActor :type Actor%20Object%20Reference)))

(event EventTick
  (params (DeltaSeconds :type Float%20%28single-precision%29)))

(fn ConstructionScript)