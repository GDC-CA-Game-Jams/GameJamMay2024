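; BP_SpriteCharacter is the player character, handling side-to-side movement and interaction with overlapping entities and NPCs.
; BeginPlay adds the IM_Player Enhanced Input context, and IA_Move drives movement along world X only.
; Two IA_Interact handlers search overlapping BP_PaperEntity and BP_PaperNPC actors, each messaging the first BPI_Interactions implementer.
; Dialogue and ShowInteractTooltip are stubs returning false, and overlap begin only prints debug text.
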(event Input|EnhancedActionEvents|EnhancedInputActionIA_Move
  (params (ActionValue :type Vector%202D%20Structure) (ElapsedSeconds :type Float%20%28double-precision%29) (TriggeredSeconds :type Float%20%28double-precision%29) (InputAction :type Input%20Action%20Object%20Reference :default "/Game/Input/Actions/IA_Move.IA_Move"))
  ;[1 1 1] allows player to move
  (Pawn|Input|AddMovementInput "1.000000,0.000000,0.000000" (.x ActionValue) false))

(event Input|EnhancedActionEvents|EnhancedInputActionIA_Interact
  (params (ActionValue :type Boolean) (ElapsedSeconds :type Float%20%28double-precision%29) (TriggeredSeconds :type Float%20%28double-precision%29) (InputAction :type Input%20Action%20Object%20Reference :default "/Game/Input/Actions/IA_Interact.IA_Interact"))
  ;[1 1 1] player checks for paper entity actor and uses interaction if implemented.
  (bind _array_element (Utilities|Array|ForEachLoopwithBreak (Collision|GetOverlappingActors "/Game/BP_PaperEntity.BP_PaperEntity_C" :!class /Script/Engine.Actor) :!label _label)
    (:LoopBody
      (if (Utilities|DoesObjectImplementInterface _array_element "/Game/BPI_Interactions.BPI_Interactions_C")
        (Class|BPIInteractions|OnInteract(Message) _array_element)
        (goto _label Break)))))

(event Input|EnhancedActionEvents|EnhancedInputActionIA_Interact
  (params (ActionValue :type Boolean) (ElapsedSeconds :type Float%20%28double-precision%29) (TriggeredSeconds :type Float%20%28double-precision%29) (InputAction :type Input%20Action%20Object%20Reference :default "/Game/Input/Actions/IA_Interact.IA_Interact"))
  (bind _array_element (Utilities|Array|ForEachLoopwithBreak (Collision|GetOverlappingActors "/Game/BP_PaperNPC.BP_PaperNPC_C" :!class /Script/Engine.Actor) :!label _label)
    (:LoopBody
      (if (Utilities|DoesObjectImplementInterface _array_element "/Game/BPI_Interactions.BPI_Interactions_C")
        (Class|BPIInteractions|OnInteract(Message) _array_element)
        (goto _label Break)))))

(event EventBeginPlay
  (bind _returnvalue (PlayerController|LocalPlayerSubsystems|GetEnhancedInputLocalPlayerSubsystem))
  ;[1 1 1] gives player the input system mapping
  (Utilities|IsValid _returnvalue
    (:Is%20Valid
      (Input|AddMappingContext _returnvalue "/Game/Input/IM_Player.IM_Player" 0 "(bIgnoreAllPressedKeysUntilRelease=True,bForceImmediately=False,bNotifyUserSettings=False)"))))

(event Collision|EventActorBeginOverlap
  (params (OtherActor :type Actor%20Object%20Reference))
  (Development|PrintString "Overlap"))

(fn ConstructionScript)

(fn Dialogue
  (params (isNPC :type BP%20Paper%20NPC%20Object%20Reference))
  (return false))

(fn ShowInteractTooltip
  (return false))