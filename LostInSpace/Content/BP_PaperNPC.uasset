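; BP_PaperNPC is an interactable NPC that starts a conversation when the player interacts with it.
; OnInteract passes IntroDialogueTable to LaunchDialogue, while the Dialogue and ShowInteractTooltip functions are stubs returning false.
; Disconnected leftover nodes hold an older approach that steps through a dialogue array in a WB_Dialogue widget and switches to UI-only input with a visible cursor.
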(event EventBeginPlay)

(event Collision|EventActorBeginOverlap
  (params (OtherActor :type Actor%20Object%20Reference)))

(event EventTick
  (params (DeltaSeconds :type Float%20%28single-precision%29)))

(event EventOnInteract
  (params (DialougeIneract :type Character%20Object%20Reference))
  (CallFunction|LaunchDialogue "/Game/DialogueSystem/IntroDialogueTable.IntroDialogueTable"))

(fn ConstructionScript)

(fn Dialogue
  (params (isNPC :type BP%20Paper%20NPC%20Object%20Reference))
  (return false))

(fn ShowInteractTooltip
  (return false))